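; BP_BlinkFloor is a floor that vanishes after a character touches it.
; A hit on the Cube binds a handler to that character's actor-hit event and starts a five-second timer for AppearFloor.
; The apparent handler, an auto-generated function, hides the Cube and disables collision; its own timer call has no event connected.
; AppearFloor restores only visibility, not collision, and the DisappearFloor timer is never run.
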(event OnComponentHit(Cube)
  (params (HitComponent :type Primitive%20Component%20Object%20Reference) (OtherActor :type Actor%20Object%20Reference) (OtherComp :type Primitive%20Component%20Object%20Reference) (NormalImpulse :type Vector :default "0, 0, 0") (Hit :type Hit%20Result%20Structure%20%28by%20ref%29))
  (bind _as캐릭터 (Utilities|Casting|CastToCharacter OtherActor))
  (Collision|BindEventtoOnActorHit _as캐릭터 (EventDispatchers|CreateEvent :!event BPBlinkFloorAutoGenFunc))
  (Utilities|Time|SetTimerbyFunctionName 0 "AppearFloor" 5.0))

(fn ConstructionScript)

(fn DisappearFloor
  (Rendering|SetVisibility (Variables|Default|GetCube) false false))

(fn AppearFloor
  (Rendering|SetVisibility (Variables|Default|GetCube) true false))

(fn BPBlinkFloorAutoGenFunc
  (params (SelfActor :type Actor%20Object%20Reference) (OtherActor :type Actor%20Object%20Reference) (NormalImpulse :type Vector) (Hit :type Hit%20Result%20Structure%20%28by%20ref%29))
  (Utilities|Time|SetTimerbyEvent 0 2.0)
  (Rendering|SetVisibility (Variables|Default|GetCube) false false)
  (Collision|SetCollisionEnabled (Variables|Default|GetCube) "NoCollision"))