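; Moving actor that slides its Cube back and forth along a relative X/Z diagonal while a linked Switch is on.
; On BeginPlay it binds to the Switch's update dispatcher, with a toggle handler that starts or stops the motion through DoPlayAndStop.
; A timeline scales the Cube's offset, and each finish flips IsRight and re-enters the branch to alternate Play and Reverse, looping until stopped.
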(event Custom|DoStop
  (bind _value (Timeline|타임라인 Stop)
    (:Update
      (Transformation|SetRelativeLocation (Variables|Default|GetCube) (* _value "100.000000,0.000000,100.000000") false false))
    (:Finished
      (Variables|Default|SetIsRight (not (Variables|Default|GetIsRight)))
      (if (Variables|Default|GetIsRight)
        (Timeline|타임라인 Play)
        (else
          (Timeline|타임라인 Reverse))))))

(event Custom|DoPlay
  (if (Variables|Default|GetIsRight) :!label _label
    (bind _value (Timeline|타임라인 Play)
      (:Update
        (Transformation|SetRelativeLocation (Variables|Default|GetCube) (* _value "100.000000,0.000000,100.000000") false false))
      (:Finished
        (Variables|Default|SetIsRight (not (Variables|Default|GetIsRight)))
        (goto _label)))
    (else
      (Timeline|타임라인 Reverse))))

(event EventBeginPlay
  (EventDispatchers|BindEventtoEventDispatcherUpdateSwitch (Variables|Default|GetSwitch) (EventDispatchers|CreateEvent :!event EventSwitchToggle)))

(fn ConstructionScript)

(fn EventSwitchToggle
  (params (Toggle :type Boolean))
  (CallFunction|DoPlayandStop Toggle))

(fn DoPlayandStop
  (params (IsPlay :type Boolean))
  (if IsPlay
    (CallFunction|DoPlay)
    (else
      (CallFunction|DoStop)))
  (return true))