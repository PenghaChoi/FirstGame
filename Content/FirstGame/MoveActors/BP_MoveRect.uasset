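; BP_MoveRect is an actor that moves its Cube around a rectangular loop in the local X-Z plane while IsPlay is true.
; Tick runs a MoveType state machine (Right, Up, Left, Down), advancing when the relative location passes each bound.
; Each direction function adds a fixed per-frame offset without delta-time scaling or sweep.
; BeginPlay binds to a Switch's update dispatcher, and EventSwitchToggle and DoPlayAndStop set IsPlay.
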(event EventBeginPlay
  (EventDispatchers|BindEventtoEventDispatcherUpdateSwitch (Variables|Default|GetSwitch) (EventDispatchers|CreateEvent :!event EventSwitchToggle)))

(event EventTick
  (params (DeltaSeconds :type Float%20%28single-precision%29))
  (if (Variables|Default|GetIsPlay)
    (switch Utilities|FlowControl|Switch|SwitchonENUM_MoveType (Variables|Default|GetMoveType)
      (:NewEnumerator0
        (CallFunction|오른쪽으로이동)
        (if (> (.x (Variables|/Script/Engine.SceneComponent|GetRelativeLocation (Variables|Default|GetCube))) 4e+02)
          (Variables|Default|SetMoveType "NewEnumerator1")))
      (:NewEnumerator1
        (CallFunction|위로이동)
        (if (> (.z (Variables|/Script/Engine.SceneComponent|GetRelativeLocation (Variables|Default|GetCube))) 4e+02)
          (Variables|Default|SetMoveType "NewEnumerator2")))
      (:NewEnumerator2
        (CallFunction|왼쪽으로이동)
        (if (< (.x (Variables|/Script/Engine.SceneComponent|GetRelativeLocation (Variables|Default|GetCube))) 0.0)
          (Variables|Default|SetMoveType "NewEnumerator3")))
      (:NewEnumerator3
        (CallFunction|아래로이동)
        (if (< (.z (Variables|/Script/Engine.SceneComponent|GetRelativeLocation (Variables|Default|GetCube))) 0.0)
          (Variables|Default|SetMoveType "NewEnumerator0"))))))

(fn ConstructionScript)

(fn 오른쪽으로이동
  (Transformation|AddRelativeLocation (Variables|Default|GetCube) "10.000000,0.000000,0.000000" false false))

(fn 위로이동
  (Transformation|AddRelativeLocation (Variables|Default|GetCube) "0.000000,0.000000,10.000000" false false))

(fn 왼쪽으로이동
  (Transformation|AddRelativeLocation (Variables|Default|GetCube) "-10.000000,0.000000,0.000000" false false))

(fn 아래로이동
  (Transformation|AddRelativeLocation (Variables|Default|GetCube) "0.000000,0.000000,-10.000000" false false))

(fn EventSwitchToggle
  (params (Toggle :type Boolean))
  (Variables|Default|SetIsPlay Toggle))

(fn DoPlayandStop
  (params (IsPlay :type Boolean))
  (Variables|Default|SetIsPlay IsPlay)
  (return true))