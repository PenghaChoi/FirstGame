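; BP_CounterSwitch is an overlap-triggered switch that counts touches and toggles a set of actors between play and stop.
; Each Cube overlap increments Count, resets it to 0 past 9, and shows it on a TextRender.
; Odd counts send play and even counts send stop to the Actors array through a BPI_PlayStop cast and DoPlayAndStop.
; Its own DoPlayAndStop is a stub that returns false.
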(event OnComponentBeginOverlap(Cube)
  (params (OverlappedComponent :type Primitive%20Component%20Object%20Reference) (OtherActor :type Actor%20Object%20Reference) (OtherComp :type Primitive%20Component%20Object%20Reference) (OtherBodyIndex :type Integer) (bFromSweep :type Boolean) (SweepResult :type Hit%20Result%20Structure%20%28by%20ref%29))
  (Utilities|FlowControl|Sequence
    (:then_0
      (CallFunction|카운트증가표시))
    (:then_1
      (if (== (Math|Integer|%(Integer) (Variables|Default|GetCount) 2) 1)
        (CallFunction|Play)
        (else
          (CallFunction|Stop))))))

(event EventBeginPlay
  (CallFunction|ShowCount))

(fn ConstructionScript)

(fn 카운트증가표시
  ;[0.15 0.15 0.15 0.5] 카운트 증가 표시
  (CallFunction|Count1Up)
  (CallFunction|Over9Count0)
  (CallFunction|ShowCount))

(fn Play
  (for _array_element (Variables|Default|GetActors)
    (bind _asbpi_play_stop (Utilities|Casting|CastToBPI_PlayStop _array_element))
    (Default|DoPlayandStop _asbpi_play_stop true)))

(fn Stop
  (for _array_element (Variables|Default|GetActors)
    (bind _asbpi_play_stop (Utilities|Casting|CastToBPI_PlayStop _array_element))
    (Default|DoPlayandStop _asbpi_play_stop false)))

(fn Count1Up
  (Variables|Default|SetCount (+ (Variables|Default|GetCount) 1)))

(fn Over9Count0
  (if (> (Variables|Default|GetCount) 9)
    (Variables|Default|SetCount 0)))

(fn ShowCount
  ;[0.15 0.15 0.15 0.5] Count를 Text Render에 표시
  (Rendering|Components|TextRender|SetText (Variables|Default|GetTextRender) (Utilities|Text|ToText(Integer) (Variables|Default|GetCount))))

(fn DoPlayandStop
  (params (IsPlay :type Boolean))
  (return false))