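; BP_CannonBall is a physics projectile that launches forward on spawn and self-destructs after five seconds if it hits nothing.
; On a sphere hit it spawns explosion particles and sound, destroys itself, and applies damage to the hit actor.
; Hit Characters also get a movement impulse from the reversed, scaled hit normal impulse, and BP_ThirdPersonCharacter targets switch to ragdoll.
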(event OnComponentHit(Sphere)
  (params (HitComponent :type Primitive%20Component%20Object%20Reference) (OtherActor :type Actor%20Object%20Reference) (OtherComp :type Primitive%20Component%20Object%20Reference) (NormalImpulse :type Vector :default "0, 0, 0") (Hit :type Hit%20Result%20Structure%20%28by%20ref%29))
  (Utilities|FlowControl|Sequence
    (:then_0
      (CallFunction|DoExplosion)
      (CallFunction|DoImpulseTarget OtherActor NormalImpulse)
      (bind _asbp_third_person_character (Utilities|Casting|CastToBP_ThirdPersonCharacter OtherActor))
      (Default|DoRagdoll _asbp_third_person_character true))
    (:then_1
      (Game|Damage|ApplyDamage OtherActor 1e+01 0 self))))

(event EventBeginPlay
  (bind _sphere (Variables|Default|GetSphere))
  (Physics|AddImpulse _sphere (* (Math|Vector|GetForwardVector _sphere) 2e+05) "None" false)
  (Utilities|FlowControl|Delay 5.0)
  (Actor|DestroyActor))

(fn ConstructionScript)

(fn DoImpulseTarget
  (params (OtherActor :type Actor%20Object%20Reference) (Normal%20Impulse :type Vector))
  (bind _as캐릭터 (Utilities|Casting|CastToCharacter OtherActor))
  (Physics|AddImpulse (Variables|/Script/Engine.Character|GetCharacterMovement _as캐릭터) (* Normal%20Impulse -2.0) false))

(fn DoExplosion
  (bind _sphere (Variables|Default|GetSphere))
  (bind _returnvalue (Transformation|GetWorldTransform _sphere))
  (Effects|SpawnEmitteratLocation "/Game/StarterContent/Particles/P_Explosion.P_Explosion" (.location _returnvalue) (.rotation _returnvalue))
  (Audio|SpawnSoundatLocation "/Game/StarterContent/Audio/Explosion_Cue.Explosion_Cue" (.location _returnvalue) "0, 0, 0" 1.0 1.0 0.0 0 0)
  (Actor|DestroyActor))